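; Lobby game mode that registers joining players and pushes server and map settings to their lobby player controllers.
; On PostLogin it records the controller, gathers PlayerStarts, reads server name and max players from the Steam game instance, then initializes that player's lobby menu.
; StartLoadingScreen tells every connected controller to show a loading screen.
; SpawnPlayer is called after login but is an empty stub, leaving the gathered spawn points unused.
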(event Custom|SpawnPlayer
  (params (Player :type Player%20Controller%20Object%20Reference)))

(event Custom|StartLoadingScreen
  (for _array_element (Variables|Default|GetConectedPlayers)
    (bind _lobbypc (Class|BPILobbyPC|LobbyPCRef(Message) _array_element))
    (Default|ShowLoadingScreen _lobbypc)))

(event EventPostLogin
  (params (NewPlayer :type Player%20Controller%20Object%20Reference))
  (bind _output_get (Variables|Default|SetConectedPlayer NewPlayer))
  (Utilities|Array|AddUnique (Variables|Default|GetConectedPlayers) _output_get)
  (bind _outactors (Actor|GetAllActorsOfClass "/Script/Engine.PlayerStart"))
  (Variables|Default|SetSpawnPoints _outactors)
  (bind _game_instane (Class|BPIGameInstance|SteamGameInstanceRef(Message) (Game|GetGameInstance)))
  (Variables|Default|SetServerName (Variables|/Game/_Main/SteamGameInstance.SteamGameInstance_C|GetServerName _game_instane))
  (Variables|Default|SetMaxPlayer (Variables|/Game/_Main/SteamGameInstance.SteamGameInstance_C|GetMaxPlayers _game_instane))
  (bind _lobbypc (Class|BPILobbyPC|LobbyPCRef(Message) (Variables|Default|GetConectedPlayer)))
  (Default|InicialSetup _lobbypc)
  (Default|SetupLobbyMenu _lobbypc (Variables|Default|GetServerName))
  (Default|UpdateLobbySettings _lobbypc (Variables|Default|GetDefault%20Map%20Image) (Variables|Default|GetDefault%20Map%20Name) (Variables|Default|GetDefault%20Map%20Time))
  (CallFunction|SpawnPlayer (Variables|Default|GetConectedPlayer)))

(fn ConstructionScript)

(fn LobbyGMref
  (return self))